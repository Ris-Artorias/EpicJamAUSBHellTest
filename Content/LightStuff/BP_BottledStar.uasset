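; BP_BottledStar is a carried light source whose glow drains while held, destroying the player character and itself when it runs out.
; Each Tick while Held, it lowers LightIntensity by a fixed frame-rate-dependent step, applies it to the PointLight and updates a percent variable intended for a UI progress bar.
; While light remains, each held Tick also overwrites the actor's Tags to remove the original pickup tag.
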(event `self.ReceiveBeginPlay`)

(event `self.ReceiveTick`
  (params (DeltaSeconds :type "Float (single-precision)"))
  ;[1 1 1] Every tick, if picked up by the player, the light intensity decreases
  (if (`self.Held`)
    (bind _output_get (set `self.LightIntensity` (- (`self.LightIntensity`) 1.0)))
    ;[1 1 1] Tried to get the UI progress bar to bind to this variable.
    (set `self.LightIntensityPercent` (/ _output_get 25000.0))
    (`LightComponent.SetIntensity` (`self.PointLight`) _output_get)
    (if (<= _output_get 0.0)
      (bind _asbp_first_person_character (cast `/Game/FirstPerson/Blueprints/BP_FirstPersonCharacter` (`GameplayStatics.GetPlayerCharacter` 0)))
      (`self.K2_DestroyActor` _asbp_first_person_character)
      (`self.K2_DestroyActor`)
      (else
        ;[1 1 1] This just deletes the original pickup tag, don't question it.
        (set `self.Tags` (`self.Tags_0`))))))

(fn `UserConstructionScript`)