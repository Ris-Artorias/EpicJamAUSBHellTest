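; AI controller for BP_Monster that runs its behavior tree and tracks whether it senses the player.
; BeginPlay caches the possessed monster, starts BT_Monster and stores the player controller as FollowTarget.
; Perception updates for BP_ThirdPersonCharacter write the sensed state to the CanSeePlayer blackboard key.
; FacePlayer is an empty event, and an interpolated yaw rotation toward the player sits disconnected and never runs.
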(event `self.ReceiveBeginPlay`
  (bind _asbp_monster (cast `/Game/Blueprints/BP_Monster` (`self.K2_GetPawn`)))
  (set `self.Monster` _asbp_monster)
  (`self.RunBehaviorTree` "/Game/Blueprints/BT_Monster.BT_Monster")
  (set `self.FollowTarget` (`GameplayStatics.GetPlayerController` 0)))

(event `self.AIPerception.OnTargetPerceptionUpdated`
  (params (Actor :type "Actor Object Reference") (Stimulus :type "AIStimulus Structure"))
  (cast `/Game/ThirdPerson/Blueprints/BP_ThirdPersonCharacter` Actor)
  (`BlackboardComponent.SetValueAsBool` (`AIBlueprintHelperLibrary.GetBlackboard` null) "CanSeePlayer" (`.bSuccessfullySensed` (break `AIStimulus` Stimulus))))

(event `Face Player`)

(fn `UserConstructionScript`)